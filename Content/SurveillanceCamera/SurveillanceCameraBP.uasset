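; Surveillance camera that tracks a tagged player in its cone, shows its alert state and shocks the player on detecting an illegal action.
; State changes recolor a dynamic decal material green, yellow or red; red shows an electric beam and spawns a burst at the player, seeking hides the beam.
; Cone overlaps set the detected player and toggle the in-range warning on player controller 5's HUD, while alarm events dispatch and display the alarm.
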(event OnComponentBeginOverlap(SurveillanceCone)
  (params (OverlappedComponent :type Primitive%20Component%20Object%20Reference) (OtherActor :type Actor%20Object%20Reference) (OtherComp :type Primitive%20Component%20Object%20Reference) (OtherBodyIndex :type Integer) (bFromSweep :type Boolean) (SweepResult :type Hit%20Result%20Structure%20%28by%20ref%29))
  (if (Actor|ActorHasTag OtherActor "Player")
    (Variables|Default|SetdetectedPlayer OtherActor)
    (Default|ShowinCameraRange (.AsMeta%20UI (Utilities|Casting|CastToMetaUI (HUD|GetHUD (Game|GetPlayerController 5)))))))

(event OnComponentEndOverlap(SurveillanceCone)
  (params (OverlappedComponent :type Primitive%20Component%20Object%20Reference) (OtherActor :type Actor%20Object%20Reference) (OtherComp :type Primitive%20Component%20Object%20Reference) (OtherBodyIndex :type Integer))
  (if (Actor|ActorHasTag OtherActor "Player")
    (Variables|Default|SetdetectedPlayer 0)
    (Default|HideMetaUI (.AsMeta%20UI (Utilities|Casting|CastToMetaUI (HUD|GetHUD (Game|GetPlayerController 5)))))))

(event EventBeginPlay
  (Rendering|SetVisibility (Variables|Default|GetElectricShock) false false)
  (bind _returnvalue (Rendering|Material|CreateDynamicMaterialInstance "/Game/SurveillanceCamera/AreaMaterial.AreaMaterial" "None" "None" :!class /Script/Engine.KismetMaterialLibrary))
  (bind _output_get (Variables|Default|SetDecalMaterial _returnvalue))
  (Rendering|Components|Decal|SetDecalMaterial (Variables|Default|GetDecal) _output_get)
  ;[1 1 1] Kamera värin vaihto
  (Rendering|Material|SetVectorParameterValue (Variables|Default|GetDecalMaterial) "Color" "(R=0.000000,G=1.000000,B=0.101418,A=1.000000)" :!class /Script/Engine.MaterialInstanceDynamic)
  (CallFunction|EndShockPlayer))

(event Collision|EventActorBeginOverlap
  (params (OtherActor :type Actor%20Object%20Reference)))

(event EventTick
  (params (DeltaSeconds :type Float%20%28single-precision%29)))

(event EventOnRaiseAlarm
  (Development|PrintString "Alarm")
  (Default|CallAlarmDispatch)
  (Default|ShowAlarm (.AsMeta%20UI (Utilities|Casting|CastToMetaUI (HUD|GetHUD (Game|GetPlayerController 5))))))

(event EventOnStateChange
  (params (newState :type CameraState%20Enum :default "kSeeking"))
  ;[1 1 1] Kamera värin vaihto
  (switch Utilities|FlowControl|Switch|SwitchonCameraState newState
    (:kSeeking
      (Rendering|Material|SetVectorParameterValue (Variables|Default|GetDecalMaterial) "Color" "(R=0.000000,G=1.000000,B=0.101418,A=1.000000)" :!class /Script/Engine.MaterialInstanceDynamic)
      (CallFunction|EndShockPlayer))
    (:kAnalyzing
      (Rendering|Material|SetVectorParameterValue (Variables|Default|GetDecalMaterial) "Color" "(R=1.000000,G=0.883292,B=0.000000,A=1.000000)" :!class /Script/Engine.MaterialInstanceDynamic))
    (:kAlarm
      (Rendering|Material|SetVectorParameterValue (Variables|Default|GetDecalMaterial) "Color" "(R=0.744792,G=0.000000,B=0.000000,A=1.000000)" :!class /Script/Engine.MaterialInstanceDynamic)
      (CallFunction|ShockPlayer))))

(fn ConstructionScript)

(fn ShockPlayer
  ;[1 1 1] Electrick shock form camera
  (Utilities|FlowControl|Sequence
    (:then_0
      (Effects|Components|ParticleSystem|SetActorParameter (Variables|Default|GetElectricShock) "EndPoint" (Variables|Default|GetdetectedPlayer))
      (Rendering|SetVisibility (Variables|Default|GetElectricShock) true false))
    (:then_1
      ;[1 1 1] Electric burst from player
      (bind _returnvalue (Game|SpawnActorfromClass "/Game/ElectricShock/ElectricBurstBP.ElectricBurstBP_C" (Transformation|GetActorTransform (Variables|Default|GetdetectedPlayer)) "Undefined" 0 0))
      (Effects|Components|ParticleSystem|SetActorParameter (Variables|/Game/ElectricShock/ElectricBurstBP.ElectricBurstBP_C|GetElecBurst _returnvalue) "Center" (Variables|Default|GetdetectedPlayer)))))

(fn EndShockPlayer
  (Rendering|SetVisibility (Variables|Default|GetElectricShock) false false))