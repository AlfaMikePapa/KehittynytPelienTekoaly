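; Behavior tree task that sends the friend robot to collect the trash object stored in the NextTrash blackboard key.
; On a successful move it clears the trash and location keys, waits briefly, asks the game instance to spawn trash and raises the robot's used capacity.
; The node that destroys the collected trash is disconnected, and only the success path finishes the task.
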(event EventReceiveExecuteAI
  (params (OwnerController :type AI%20Controller%20Object%20Reference) (ControlledPawn :type Pawn%20Object%20Reference))
  (bind _blackboard (Variables|/Script/AIModule.AIController|GetBlackboard OwnerController))
  (bind _astrash_blueprint (Utilities|Casting|CastToTrash_Blueprint (AI|Components|Blackboard|GetValueasObject _blackboard (Utilities|Name|MakeLiteralName "NextTrash"))))
  (AI|AIMoveTo ControlledPawn "0, 0, 0" _astrash_blueprint 5e+01 false
    (:OnSuccess
      ;[1 1 1] Destroy "collected" trash
      (bind _astrash_blueprint_2 (Utilities|Casting|CastToTrash_Blueprint (AI|Components|Blackboard|GetValueasObject _blackboard (Utilities|Name|MakeLiteralName "NextTrash"))))
      ;[1 1 1] Mahd turha
      (AI|Components|Blackboard|ClearValue _blackboard (Utilities|Name|MakeLiteralName "NextCollectLocation"))
      (AI|Components|Blackboard|ClearValue _blackboard (Utilities|Name|MakeLiteralName "NextTrash"))
      (Utilities|FlowControl|Delay 0.5)
      (bind _asescape_in_space_game_instance (Utilities|Casting|CastToEscapeInSpaceGameInstance (Game|GetGameInstance)))
      (Default|CallSpawnTrash _asescape_in_space_game_instance)
      (bind _asfriend_robot_bp (Utilities|Casting|CastToFriendRobot_BP ControlledPawn))
      (Variables|/Game/Blueprints/FriendRobot_BP.FriendRobot_BP_C|SetTrashCapacityUsed _asfriend_robot_bp (+ (Variables|/Game/Blueprints/FriendRobot_BP.FriendRobot_BP_C|GetTrashCapacityUsed _asfriend_robot_bp) 0.1))
      (AI|BehaviorTree|FinishExecute true))))